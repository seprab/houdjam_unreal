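; Poison zone actor that grows into place, slowly shrinks, and damages the player standing inside it.
; Tick scales it up to full size, then a self-calling delayed event shrinks it each second, with no destroy step.
; Escalar clamps X and Y from the current X scale and forces Z to zero.
; Mesh overlaps toggle PlayerInside, which keeps a delayed damage loop running on the JuadorTercera character.
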(event `self.ReceiveTick`
  (params (DeltaSeconds :type "Float (single-precision)"))
  ;[1 1 1] Escalado Inicial
  (if (not (`self.iScalation`))
    (`self.Escalar` 0.05)
    (if (>= (.x (`SceneComponent.K2_GetComponentScale` (`self.DefaultSceneRoot`))) 1.0)
      (set `self.iScalation` true)
      (`KismetSystemLibrary.Delay` 1.0)
      (`self.AchicadoConstante`))))

(event `AchicadoConstante`
  ;[1 1 1] Achicado constante
  (`self.Escalar` -0.01)
  (`KismetSystemLibrary.Delay` 1.0)
  (`self.AchicadoConstante`))

(event `DanarJugador`
  ;[1 1 1] Evento cuando el jugado entra y sale para quitarle vida
  (bind _asjuador_tercera (cast `/Game/Blueprints/JuadorTercera` (stale `self.StaticMesh.OnComponentBeginOverlap` OtherActor)))
  (`/Game/Blueprints/JuadorTercera.Damage` _asjuador_tercera 5.0)
  (`KismetSystemLibrary.Delay` 0.5)
  (if (`self.playerInside`)
    (`self.DanarJugador`)))

(event `self.StaticMesh.OnComponentBeginOverlap`
  (params (OverlappedComponent :type "PrimitiveComponent Object Reference") (OtherActor :type "Actor Object Reference") (OtherComp :type "PrimitiveComponent Object Reference") (OtherBodyIndex :type Integer) (bFromSweep :type Boolean) (SweepResult :type "HitResult Structure (by ref)"))
  ;[1 1 1] Evento cuando el jugado entra y sale para quitarle vida
  (set `self.playerInside` true)
  (`self.DanarJugador`))

(event `self.StaticMesh.OnComponentEndOverlap`
  (params (OverlappedComponent :type "PrimitiveComponent Object Reference") (OtherActor :type "Actor Object Reference") (OtherComp :type "PrimitiveComponent Object Reference") (OtherBodyIndex :type Integer))
  ;[1 1 1] Evento cuando el jugado entra y sale para quitarle vida
  (set `self.playerInside` false))

(fn `Escalar`
  (params (valor :type "Float (double-precision)"))
  (bind _returnvalue (`KismetMathLibrary.FClamp` (+ valor (.x (`SceneComponent.K2_GetComponentScale` (`self.DefaultSceneRoot`))))))
  (`SceneComponent.SetWorldScale3D` (`self.DefaultSceneRoot`) (`KismetMathLibrary.MakeVector` _returnvalue _returnvalue)))

(fn `UserConstructionScript`)