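; Meteorite-style eye projectile that gets a random TipoMeteorito and launches itself at the player from its construction script.
; The first hit plays a fracture animation and damages and pushes a struck JuadorTercera.
; Damage types destroy themselves after a delay, while others reveal a crystal.
; Once the shrink timer finishes, overlapping the crystal heals, changes speed or enlarges the player; the danger-zone reducer type has no pickup effect here.
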(event `Disparar`
  (bind _destructioncollider (`self.DestructionCollider`))
  ;[1 1 1] Disparar
  (`PrimitiveComponent.AddImpulse` _destructioncollider (* (`KismetMathLibrary.Normal` (`KismetMathLibrary.GetForwardVector` (`KismetMathLibrary.FindLookAtRotation` (`SceneComponent.K2_GetComponentLocation` _destructioncollider) (`self.K2_GetActorLocation` (`GameplayStatics.GetPlayerPawn` 0))))) (`KismetMathLibrary.RandomFloatInRange` 2222222.0 3333333.0)) "None" false))

(event `MostrarCristal`
  (bind _cristal (`self.Cristal`))
  ;[1 1 1] Mostrar cristal y esconder ojo
  (`SceneComponent.SetWorldScale3D` _cristal (4.0 4.0 4.0))
  (`SceneComponent.K2_SetWorldLocation` _cristal (`SceneComponent.K2_GetComponentLocation` (`self.DestructionCollider`)) false true)
  (`SceneComponent.K2_SetWorldRotation` :`self` _cristal :`bTeleport` true)
  (`PrimitiveComponent.SetCollisionEnabled` _cristal "QueryAndPhysics"))

(event `ColisionEsfera`
  (bind _destructioncollider (`self.DestructionCollider`))
  (`SceneComponent.SetWorldScale3D` _destructioncollider (0.0 0.0 0.0))
  (`ActorComponent.Deactivate` _destructioncollider)
  (set `self.animFinished` true))

(event `self.DestructionCollider.OnComponentHit`
  (params (HitComponent :type "PrimitiveComponent Object Reference") (OtherActor :type "Actor Object Reference") (OtherComp :type "PrimitiveComponent Object Reference") (NormalImpulse :type "Vector Structure") (Hit :type "HitResult Structure (by ref)"))
  (bind _destructioncollider (`self.DestructionCollider`))
  ;[1 1 1] Evento Destruccion ojo
  (if (not (`self.animPlayed`))
    (`SkeletalMeshComponent.PlayAnimation` (`self.SkeletalMesh`) "/Game/Geometry/Meshes/fracture_002_Anim.fracture_002_Anim" false)
    (`PrimitiveComponent.SetSimulatePhysics` _destructioncollider false)
    (`PrimitiveComponent.SetCollisionEnabled` _destructioncollider "NoCollision")
    (set `self.animPlayed` true)
    (`|ExecutionSequence`
      (:`then_0`
        (switch `/Game/Blueprints/TipoMeteorito` (`self.tipo`)
          (:`NewEnumerator0`
            (`KismetSystemLibrary.Delay` 4.0)
            (`self.Destroy Object`))
          (:`NewEnumerator1`
            (`self.MostrarCristal` :!label _label))
          (:`NewEnumerator2`
            (goto _label))
          (:`NewEnumerator4`
            (goto _label))
          (:`NewEnumerator3`
            (goto _label))
          (:`NewEnumerator5`
            (goto _label))))
      (:`then_1`
        (`KismetSystemLibrary.K2_SetTimerDelegate` (delegate `ColisionEsfera`) 2.0))
      (:`then_2`
        (bind _asjuador_tercera (cast `/Game/Blueprints/JuadorTercera` OtherActor))
        (`/Game/Blueprints/JuadorTercera.Damage` _asjuador_tercera 25.0)
        (`/Game/Blueprints/JuadorTercera.AddImpulse` _asjuador_tercera (`self.iLocation`))))))

(event `self.Cristal.OnComponentBeginOverlap`
  (params (OverlappedComponent :type "PrimitiveComponent Object Reference") (OtherActor :type "Actor Object Reference") (OtherComp :type "PrimitiveComponent Object Reference") (OtherBodyIndex :type Integer) (bFromSweep :type Boolean) (SweepResult :type "HitResult Structure (by ref)"))
  (bind _returnvalue (`KismetMathLibrary.RandomFloatInRange` 4.0 8.0))
  (bind _returnvalue_2 (`KismetMathLibrary.RandomFloatInRange` 200.0 400.0))
  (bind _tipo (`self.tipo`))
  ;[1 1 1] Trigger Event Cristal
  (if (`self.animFinished`)
    (`KismetSystemLibrary.PrintString` (`|GetEnumeratorNameAsString` _tipo))
    (switch `/Game/Blueprints/TipoMeteorito` _tipo
      (:`NewEnumerator1`
        (bind _asjuador_tercera (cast `/Game/Blueprints/JuadorTercera` OtherActor))
        (`/Game/Blueprints/JuadorTercera.Heal` _asjuador_tercera 10.0))
      (:`NewEnumerator4`
        (bind _asjuador_tercera_2 (cast `/Game/Blueprints/JuadorTercera` OtherActor))
        (`/Game/Blueprints/JuadorTercera.ModifySpeed` _asjuador_tercera_2 (* -1 _returnvalue_2) _returnvalue))
      (:`NewEnumerator3`
        (bind _asjuador_tercera_3 (cast `/Game/Blueprints/JuadorTercera` OtherActor))
        (`/Game/Blueprints/JuadorTercera.ModifySpeed` _asjuador_tercera_3 _returnvalue_2 _returnvalue))
      (:`NewEnumerator5`
        (bind _asjuador_tercera_4 (cast `/Game/Blueprints/JuadorTercera` OtherActor))
        (`/Game/Blueprints/JuadorTercera.AgrandarPJ` _asjuador_tercera_4 (+ (`/Game/Blueprints/JuadorTercera.iScale` _asjuador_tercera_4) 2) true)))
    (`self.K2_DestroyActor`)))

(event `Destroy Object`
  ;[1 1 1] DestruiObjeto
  (`self.K2_DestroyActor`))

(fn `UserConstructionScript`
  (bind _cristal (`self.Cristal`))
  (`|ExecutionSequence`
    (:`then_0`
      (bind _output_get (set `self.tipo` (cast `/Game/Blueprints/TipoMeteorito` (`KismetMathLibrary.Conv_IntToByte` (`KismetMathLibrary.RandomInteger` (enumcount `/Game/Blueprints/TipoMeteorito`))))))
      (switch `/Game/Blueprints/TipoMeteorito` _output_get))
    (:`then_1`
      (`SceneComponent.SetWorldScale3D` _cristal (4.0 4.0 4.0))
      (`PrimitiveComponent.SetCollisionEnabled` _cristal "NoCollision")
      (set `self.iLocation` (`self.K2_GetActorLocation`)))
    (:`then_2`
      (`self.Disparar`))))